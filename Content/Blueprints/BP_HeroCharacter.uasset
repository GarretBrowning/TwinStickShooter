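; Player hero for a twin-stick shooter that moves on world axes and spawns a laser rifle on its socket plus the HUD.
; Look axes past a deadzone set control rotation and fire after a short delay, otherwise releasing the trigger.
; Shotgun burst and damage boost pickups toggle timed rifle flags, both using the damage boost HUD indicator.
; On death, it disables input, waits, asks the game mode to respawn, then destroys itself and the rifle.
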(event Custom|ShotgunSpread
  ;[1 0.8874 0] Activates Upon Shotgun Burst Powerup Pickup. Sets the Value of Is Damage Boosted to True and Shows the HUD Indicator (Bottom Left Corner). After a Set Duration (Delay), Reset `Is Damage Boosted` Value to False and Hide HUD Indicator.
  (Variables|/Game/Blueprints/BP_LaserRifle.BP_LaserRifle_C|SetbIsShotgunBurstActive (Variables|Default|GetLaserRifle) true)
  (Default|ResetTimer (Variables|Default|GetLaserRifle))
  (Widget|SetVisibility (Variables|/Game/Blueprints/WBP_TwinStickHUD.WBP_TwinStickHUD_C|GetDamageBoostStatus (stale EventBeginPlay _returnvalue_2)) "Visible")
  (Audio|PlaySound2D "/Game/Sounds/Powerup_Pickup_DamageBoost.Powerup_Pickup_DamageBoost" 1.0 1.0 0.0 0 0)
  (Utilities|FlowControl|Delay 8.0) ; Powerup Lasts for 8 Seconds.
  (Variables|/Game/Blueprints/BP_LaserRifle.BP_LaserRifle_C|SetbIsShotgunBurstActive (Variables|Default|GetLaserRifle) false)
  (Default|ResetTimer (Variables|Default|GetLaserRifle))
  (Widget|SetVisibility (Variables|/Game/Blueprints/WBP_TwinStickHUD.WBP_TwinStickHUD_C|GetDamageBoostStatus (stale EventBeginPlay _returnvalue_2)) "Hidden"))

(event Custom|DamageBoost
  ;[0 0.6406 0.08408] Activates Upon Damage Boost Powerup Pickup. Sets the Value of Is Damage Boosted to True and Shows the HUD Indicator (Bottom Left Corner). After a Set Duration (Delay), Reset `Is Damage Boosted` Value to False and Hide HUD Indicator.
  (Variables|/Game/Blueprints/BP_LaserRifle.BP_LaserRifle_C|SetbIsDamageBoosted (Variables|Default|GetLaserRifle) true)
  (Default|ResetTimer (Variables|Default|GetLaserRifle))
  (Widget|SetVisibility (Variables|/Game/Blueprints/WBP_TwinStickHUD.WBP_TwinStickHUD_C|GetDamageBoostStatus (stale EventBeginPlay _returnvalue_2)) "Visible")
  (Audio|PlaySound2D "/Game/Sounds/Powerup_Pickup_DamageBoost.Powerup_Pickup_DamageBoost" 1.0 1.0 0.0 0 0)
  (Utilities|FlowControl|Delay 8.0) ; Powerup Lasts for 8 Seconds.
  (Variables|/Game/Blueprints/BP_LaserRifle.BP_LaserRifle_C|SetbIsDamageBoosted (Variables|Default|GetLaserRifle) false)
  (Default|ResetTimer (Variables|Default|GetLaserRifle))
  (Widget|SetVisibility (Variables|/Game/Blueprints/WBP_TwinStickHUD.WBP_TwinStickHUD_C|GetDamageBoostStatus (stale EventBeginPlay _returnvalue_2)) "Hidden"))

(event EventBeginPlay
  (bind _mesh (Variables|Character|GetMesh))
  (Utilities|FlowControl|Sequence
    (:then_0
      ;[0 0.6406 0.08408] Setting Up the Laser Rifle to be Attached to the Hero Character.
      (bind _returnvalue (Game|SpawnActorfromClass "/Game/Blueprints/BP_LaserRifle.BP_LaserRifle_C" (Transformation|GetWorldTransform _mesh) "Undefined" 0 0))
      (bind _output_get (Variables|Default|SetLaserRifle _returnvalue))
      (Transformation|AttachComponentToComponent _output_get _mesh "RifleSocket" "SnapToTarget" "SnapToTarget" "KeepWorld" true))
    (:then_1
      ;[0 0.6406 0.08408] Setting the GameMode to be TwinStickMode.
      (bind _asbp_twin_stick_mode (Utilities|Casting|CastToBP_TwinStickMode (Game|GetGameMode)))
      (Variables|Default|SetGameMode _asbp_twin_stick_mode))
    (:then_2
      ;[0 0.6406 0.08408] Setting Up the HUD to the Viewport.
      (bind _returnvalue_2 (UserInterface|CreateWidget "/Game/Blueprints/WBP_TwinStickHUD.WBP_TwinStickHUD_C"))
      (UserInterface|Viewport|AddtoViewport _returnvalue_2 0))))

(event EventAffectHealth
  (params (Delta :type Float%20%28single-precision%29))
  ;[0 0.6406 0.08408] Calculates the Health for the Hero Character. If the Hero Character Dies, Disable Any Further Input, Release The Trigger of the Laser Rifle, and Respawn the Player.
  (Class|BaseCharacter|CalculateHealth Delta)
  (if (Variables|Default|GetbIsDead)
    (Input|DisableInput 0)
    (Default|ReleaseTrigger (Variables|Default|GetLaserRifle))
    (Utilities|FlowControl|Delay 3.0) ; Delay used for death animation purposes.
    (Default|RespawnPlayer (Variables|Default|GetGameMode))
    (Actor|DestroyActor (Variables|Default|GetLaserRifle))))

(event Input|AxisEvents|InputAxisMoveUp
  (params (AxisValue :type Float%20%28single-precision%29))
  ;[0 0.6406 0.08408] Moving the Hero Character Using X as the Forward (Up) Direction and Y as the Side (Right) Direction.
  (Pawn|Input|AddMovementInput "1.000000, 0, 0" AxisValue false))

(event Input|AxisEvents|InputAxisMoveRight
  (params (AxisValue :type Float%20%28single-precision%29))
  ;[0 0.6406 0.08408] Moving the Hero Character Using X as the Forward (Up) Direction and Y as the Side (Right) Direction.
  (Pawn|Input|AddMovementInput "0.000000,1.000000, 0" AxisValue false))

(event Input|AxisEvents|InputAxisLookUp
  (params (AxisValue :type Float%20%28single-precision%29))
  (bind _laserrifle (Variables|Default|GetLaserRifle))
  ;[0 0.6406 0.08408] Controlling the Hero Character's Rotation Using LookUp and LookRight Input Events. When The Input Value is Greater Than 0.25, We Will Set Hero Character's Rotation to the New Value. If the Hero Character Rotates Then They Will Fire Their Laser Rifle; Otherwise, They Will Cease Firing.
  (if (> (Math|Vector|VectorLength (Math|Vector|MakeVector AxisValue (stale Input|AxisEvents|InputAxisLookRight AxisValue) 0.0)) 0.25)
    (if (not (Variables|Default|GetbIsDead)) ; Checks to make sure the Hero Character cannot fire their rifle when dead.
      (Pawn|SetControlRotation (Pawn|GetController) (Math|Conversions|RotationFromXVector (Math|Vector|MakeVector AxisValue (stale Input|AxisEvents|InputAxisLookRight AxisValue) 0.0)))
      (Utilities|FlowControl|Delay 0.2) ; Input delay to ensure all of the laser bullets fire towards the desired direction.
      (Default|PullTrigger _laserrifle)
      (else
        (Default|ReleaseTrigger _laserrifle :!label _label)))
    (else
      (goto _label))))

(event Input|AxisEvents|InputAxisLookRight
  (params (AxisValue :type Float%20%28single-precision%29))
  (bind _laserrifle (Variables|Default|GetLaserRifle))
  ;[0 0.6406 0.08408] Controlling the Hero Character's Rotation Using LookUp and LookRight Input Events. When The Input Value is Greater Than 0.25, We Will Set Hero Character's Rotation to the New Value. If the Hero Character Rotates Then They Will Fire Their Laser Rifle; Otherwise, They Will Cease Firing.
  (if (> (Math|Vector|VectorLength (Math|Vector|MakeVector (stale Input|AxisEvents|InputAxisLookUp AxisValue) AxisValue 0.0)) 0.25)
    (if (not (Variables|Default|GetbIsDead)) ; Checks to make sure the Hero Character cannot fire their rifle when dead.
      (Pawn|SetControlRotation (Pawn|GetController) (Math|Conversions|RotationFromXVector (Math|Vector|MakeVector (stale Input|AxisEvents|InputAxisLookUp AxisValue) AxisValue 0.0)))
      (Utilities|FlowControl|Delay 0.2) ; Input delay to ensure all of the laser bullets fire towards the desired direction.
      (Default|PullTrigger _laserrifle)
      (else
        (Default|ReleaseTrigger _laserrifle :!label _label)))
    (else
      (goto _label))))

(fn ConstructionScript)