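; Laser rifle projectile that damages non-friendly actors on overlap.
; On BeginPlay it reads the player hero's LaserRifle and, if damage boosted, swaps its color, light, sparks and scale and sets a boosted damage value.
; On overlap it sends a negative health change through BPI_Damageable, then spawns sparks and destroys itself.
; Non-damageable actors also trigger sparks and destruction, while Friendly-tagged damageable actors are ignored.
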(event Collision|EventActorBeginOverlap
  (params (OtherActor :type Actor%20Object%20Reference))
  (bind _returnvalue (Transformation|GetActorTransform))
  ;[0 0.6406 0.08408] When the Projectile Overlaps a Pawn, It Checks to See if it has the BPI_Damageable Interface. If it does and the Actor does NOT have the Friendly Tag, then we Affect its Health by `Damage` Amount and Sparks Spawn at the Point of Overlap; Afterwards we Destroy the Projectile. If the Actor does NOT Implement the BPI_Damageable Inteface, then we Immediately Destroy the Projectile.
  (if (Utilities|DoesObjectImplementInterface OtherActor "/Game/Blueprints/BPI_Damageable.BPI_Damageable_C")
    (if (not (Actor|ActorHasTag OtherActor "Friendly"))
      (Class|BPIDamageable|AffectHealth(Message) OtherActor (Variables|Default|GetDamage))
      (Effects|SpawnEmitteratLocation (Variables|Default|GetLaserSparks) (.location _returnvalue) (.rotation _returnvalue) :!label _label)
      (Actor|DestroyActor))
    (else
      (goto _label))))

(event EventBeginPlay
  ;[0 0.6406 0.08408] At the Beginning of the Projectile's Life, Checks to See if the Laser Rifle is Damage Boosted. If True, Changes the BaseColor, Light Color, Laser Sparks, and Relative Scale to the Projectile, as well as, Increasing the Damage.
  (bind _asbp_hero_character (Utilities|Casting|CastToBP_HeroCharacter (Game|GetPlayerCharacter 0)))
  (if (Variables|/Game/Blueprints/BP_LaserRifle.BP_LaserRifle_C|GetbIsDamageBoosted (Variables|/Game/Blueprints/BP_HeroCharacter.BP_HeroCharacter_C|GetLaserRifle _asbp_hero_character))
    (Rendering|Material|SetVectorParameterValueonMaterials (Variables|Default|GetLaserMesh) "BaseColor" (Math|Conversions|ToVector(LinearColor) (Variables|Default|GetDamageBoostLaserColor)))
    (Rendering|Components|Light|SetLightColor (Variables|Default|GetLaserLight) (Variables|Default|GetDamageBoostLightColor) true)
    (Variables|Default|SetDamage -5e+01) ; -50.0 Will Ensure an Enemy Character Dies in 2 Hits.
    (Variables|Default|SetLaserSparks "/Game/StarterContent/Particles/P_LaserSparks_DamageBoosted.P_LaserSparks_DamageBoosted")
    (Transformation|SetRelativeScale3D (Variables|Default|GetLaserMesh) "0.600000,0.210000,0.210000")))

(fn ConstructionScript)