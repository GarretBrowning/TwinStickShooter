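; BP_EnemyCharacter is a twin-stick game enemy that hurts the hero on contact and awards score when killed.
; Overlapping the hero starts a looping timer that deals damage at its attack rate until the overlap ends.
; AffectHealth updates health; on death it adds score, ignores Pawn and WorldDynamic collision, detaches the controller and destroys itself after an animation delay.
; Its construction script tints the body through a dynamic material instance.
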(event Custom|DamageHero
  ;[0 0.6406 0.08408] Damages the Hero Character by 'Damage' Amount
  (Default|AffectHealth (Variables|Default|GetHero) (Variables|Default|GetDamage)))

(event Collision|EventActorBeginOverlap
  (params (OtherActor :type Actor%20Object%20Reference))
  ;[0 0.6406 0.08408] When The Enemy Character Overlaps the Hero Character; Damage Hero (at a Rate of Attacks Per Second)
  (bind _asbp_hero_character (Utilities|Casting|CastToBP_HeroCharacter OtherActor))
  (Variables|Default|SetHero _asbp_hero_character)
  (Utilities|Time|SetTimerbyFunctionName 0 "DamageHero" (/ 1.0 (Variables|Default|GetAttacksPerSecond)) true))

(event Collision|EventActorEndOverlap
  (params (OtherActor :type Actor%20Object%20Reference))
  ;[0 0.6406 0.08408] When the Enemy Character Stops Overlapping the Hero Character; Stop Damaging The Hero Character (Clear The DamageHero Timer).
  (if (== OtherActor (Variables|Default|GetHero))
    (Utilities|Time|ClearTimerbyFunctionName 0 "DamageHero")))

(event EventAffectHealth
  (params (Delta :type Float%20%28single-precision%29))
  ;[0 0.6406 0.08408] Calculates The Enemy Character's Health and Adds the Delta Amount to the Total Health. If the Enemy Character is Dead the Score Gets Increased, The Collision Response is Set to Ignore, and Destroys the Actor.
  (Class|BaseCharacter|CalculateHealth Delta)
  (if (Variables|Default|GetbIsDead)
    (bind _asbp_twin_stick_mode (Utilities|Casting|CastToBP_TwinStickMode (Game|GetGameMode)))
    (Default|IncrementScore _asbp_twin_stick_mode (Variables|Default|GetScore))
    (Collision|SetCollisionResponsetoChannel (Variables|Default|GetCapsuleComponent) "ECC_WorldDynamic" "ECR_Ignore")
    (Collision|SetCollisionResponsetoChannel (Variables|Default|GetDamageVolume) "ECC_Pawn" "ECR_Ignore")
    (Class|Pawn|DetachfromControllerPendingDestroy)
    (Utilities|FlowControl|Delay 3.0) ; Delay the Death by 3 Seconds for Animation Purposes
    (Actor|DestroyActor)))

(fn ConstructionScript
  ;[0 0.6406 0.08408] Creating a Dynamic Material Instance for our EnemyCharacter Which Sets The New Value of BodyColor To Red.
  (bind _returnvalue (Rendering|Material|CreateDynamicMaterialInstance (Variables|Character|GetMesh) 0 0 "None" :!class /Script/Engine.PrimitiveComponent))
  (bind _output_get (Variables|Default|SetMI_DynamicMaterial _returnvalue))
  (Rendering|Material|SetVectorParameterValue _output_get "BodyColor" (Variables|Default|GetColor) :!class /Script/Engine.MaterialInstanceDynamic))