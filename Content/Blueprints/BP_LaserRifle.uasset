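; Laser rifle Blueprint that auto-fires BP_Projectile actors from its projectile spawn point while the trigger is held.
; PullTrigger passes a DoOnce to fire immediately and start a looping Fire timer; ReleaseTrigger clears the timer and resets the DoOnce.
; Fire picks its attached sound by IsDamageBoosted.
; ResetTimer sets a slower fire rate when boosted, faster otherwise, and restarts the timer without checking trigger state.
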(event Custom|PullTrigger
  ;[0 0.6406 0.08408] PullTrigger Will Execute the Fire Event Once and Will Repeat Based on the Value of ShotsFiredPerSecond.
  (Utilities|FlowControl|DoOnce false
    (:Completed
      (CallFunction|Fire)
      (bind _returnvalue (Utilities|Time|SetTimerbyFunctionName 0 "Fire" (/ 1.0 (Variables|Default|GetShotsFiredPerSecond)) true))
      (Variables|Default|SetFireTimer _returnvalue))))

(event Custom|ReleaseTrigger
  ;[0 0.6406 0.08408] ReleaseTrigger Will Reset the Timer of Fire so it is Ready to be Called Again.
  (Utilities|Time|ClearTimerbyFunctionName 0 "Fire")
  ;[0 0.6406 0.08408] PullTrigger Will Execute the Fire Event Once and Will Repeat Based on the Value of ShotsFiredPerSecond.
  (Utilities|FlowControl|DoOnce false) ; enters at Reset
)

(event Custom|Fire
  (bind _riflemesh (Variables|Default|GetRifleMesh))
  ;[0 0.6406 0.08408] Fires a Laser Projectile from the Projectile Spawn Point's Transform Location. Fires Off a Sound Effect Based on Whether the Laser Rifle is Damage Boosted or Not.
  (if (Variables|Default|GetbIsDamageBoosted)
    (Audio|SpawnSoundAttached "/Game/Sounds/LaserBlast_DamageBoosted_Cue.LaserBlast_DamageBoosted_Cue" _riflemesh "None" "0, 0, 0" "0, 0, 0" "KeepRelativeOffset" false 1.0 1.0 0.0 0 0) ; Sound from Zapsplat.com
    (else
      (Audio|SpawnSoundAttached "/Game/Sounds/LaserBlast_Cue.LaserBlast_Cue" _riflemesh "None" "0, 0, 0" "0, 0, 0" "KeepRelativeOffset" false 1.0 1.0 0.0 0 0) ; Sound from Zapsplat.com
    ))
  (Game|SpawnActorfromClass "/Game/Blueprints/BP_Projectile.BP_Projectile_C" (Transformation|GetWorldTransform (Variables|Default|GetProjectileSpawnPoint)) "Undefined" 0 0))

(event Custom|ResetTimer
  ;[0 0.6406 0.08408] Resets the Timer for the Fire Function Based on Whether the Laser Rifle is Damage Boosted. This Will Set a New Value For Shots Fired Per Second, Clear the Timer, and Set a New Timer for the Fire Function to Use.
  (if (Variables|Default|GetbIsDamageBoosted)
    (bind _output_get (Variables|Default|SetShotsFiredPerSecond 2.5))
    (Utilities|Time|ClearandInvalidateTimerbyHandle (Variables|Default|GetFireTimer))
    (bind _returnvalue (Utilities|Time|SetTimerbyFunctionName 0 "Fire" (/ 1.0 _output_get) true))
    (Variables|Default|SetFireTimer _returnvalue)
    (else
      (bind _output_get_2 (Variables|Default|SetShotsFiredPerSecond 6.0))
      (Utilities|Time|ClearandInvalidateTimerbyHandle (Variables|Default|GetFireTimer))
      (bind _returnvalue_2 (Utilities|Time|SetTimerbyFunctionName 0 "Fire" (/ 1.0 _output_get_2) true))
      (Variables|Default|SetFireTimer _returnvalue_2))))

(fn ConstructionScript)