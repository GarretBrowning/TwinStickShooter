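; BP_Powerup_ShotgunBurst is a respawning potion pickup that gives the hero character a shotgun spread.
; Overlapping its collision sphere casts to BP_HeroCharacter and calls ShotgunSpread on it.
; The glass, potion and glow then toggle invisible, and collision is disabled on the sphere and potion meshes.
; After a fixed delay, visibility toggles back and collision returns to query and physics, making the pickup available again.
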(event OnComponentBeginOverlap(SphereCollision)
  (params (OverlappedComponent :type Primitive%20Component%20Object%20Reference) (OtherActor :type Actor%20Object%20Reference) (OtherComp :type Primitive%20Component%20Object%20Reference) (OtherBodyIndex :type Integer) (bFromSweep :type Boolean) (SweepResult :type Hit%20Result%20Structure%20%28by%20ref%29))
  ;[1 0.8874 0] When the Hero Character Overlaps the Powerup, Activates Damage Boost, Toggles the Visibility (Powerup Dissapears) and Set the Collision to No Collision (Can be Passed Through). After a Delay, Toggle the Visibility and Set the Collision Back to their Default States.
  (bind _asbp_hero_character (Utilities|Casting|CastToBP_HeroCharacter OtherActor))
  (Default|ShotgunSpread _asbp_hero_character)
  (Rendering|ToggleVisibility (Variables|Default|GetPotionGlass) false)
  (Collision|SetCollisionEnabled (Variables|Default|GetPotionGlass) "NoCollision")
  (Utilities|FlowControl|Delay 1e+01) ; How Long it Takes for the Powerup Spawns After Activation.
  (Rendering|ToggleVisibility (Variables|Default|GetGlow) false)
  (Collision|SetCollisionEnabled (Variables|Default|GetSphereCollision) "QueryAndPhysics"))

(fn ConstructionScript)